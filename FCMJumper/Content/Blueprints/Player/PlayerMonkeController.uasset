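; Player controller that turns Enhanced Input actions into movement, jumping and camera look for the possessed Monke pawn.
; BeginPlay adds the main mapping context.
; Move rotates the 2D input by the pawn camera's full world rotation and feeds it to movement input, scaled by Monke's Speed.
; Jump works on any Character, while CameraTurn applies TurnRate-scaled pitch and yaw to a Monke.
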(event `self.ReceiveBeginPlay`
  (message `EnhancedInputSubsystemInterface.AddMappingContext` (pcsubsystem `EnhancedInputLocalPlayerSubsystem` self) "/Game/Input/MainContext.MainContext" 0 (struct)))

(event `EnhancedInput|/Game/Input/Actions/Move`
  (params (ActionValue :type "Vector2D Structure") (ElapsedSeconds :type "Float (double-precision)") (TriggeredSeconds :type "Float (double-precision)") (InputAction :type "InputAction Object Reference" :default "/Game/Input/Actions/Move.Move"))
  (bind _returnvalue (`self.K2_GetPawn`))
  (:`Triggered`
    (bind _asmonke (cast `/Game/Blueprints/Characters/Monke` _returnvalue))
    (`Pawn.AddMovementInput` _returnvalue (`KismetMathLibrary.GreaterGreater_VectorRotator` (`KismetMathLibrary.Conv_Vector2DToVector` ActionValue) (`SceneComponent.K2_GetComponentRotation` (`/Game/Blueprints/Characters/Monke.Camera` _asmonke))) (`/Game/Blueprints/Characters/Monke.Speed` _asmonke) false)))

(event `EnhancedInput|/Game/Input/Actions/Jump`
  (params (ActionValue :type Boolean) (ElapsedSeconds :type "Float (double-precision)") (TriggeredSeconds :type "Float (double-precision)") (InputAction :type "InputAction Object Reference" :default "/Game/Input/Actions/Jump.Jump"))
  (:`Triggered`
    (bind _ascharacter (cast `Character` (`self.K2_GetPawn`)))
    (`Character.Jump` _ascharacter)))

(event `EnhancedInput|/Game/Input/Actions/CameraTurn`
  (params (ActionValue :type "Vector2D Structure") (ElapsedSeconds :type "Float (double-precision)") (TriggeredSeconds :type "Float (double-precision)") (InputAction :type "InputAction Object Reference" :default "/Game/Input/Actions/CameraTurn.CameraTurn"))
  (bind (_x _y) (`KismetMathLibrary.BreakVector2D` (`KismetMathLibrary.Conv_VectorToVector2D` (* ActionValue (`self.TurnRate`)))))
  (:`Triggered`
    (bind _asmonke (cast `/Game/Blueprints/Characters/Monke` (`self.K2_GetPawn`)))
    (`Pawn.AddControllerPitchInput` _asmonke _y)
    (`Pawn.AddControllerYawInput` _asmonke _x)))

(fn `UserConstructionScript`)